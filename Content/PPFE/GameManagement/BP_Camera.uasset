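; BP_Camera is a player-input-driven camera pawn that moves through the world, apparently still work in progress.
; Tick offsets it by IA_MoveForward and IA_MoveSide values along forward X and right Y components, at a fixed step not scaled by delta time.
; IA_MoveForward events also add constant forward and right movement input, with debug prints.
; BeginPlay casts the controller to PC_Player but does nothing with it.
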(event Input|EnhancedActionEvents|EnhancedInputActionIA_MoveForward
  (params (ActionValue :type Float%20%28double-precision%29) (ElapsedSeconds :type Float%20%28double-precision%29) (TriggeredSeconds :type Float%20%28double-precision%29) (InputAction :type Input%20Action%20Object%20Reference :default "/Game/PPFE/Inputs/IA_MoveForward.IA_MoveForward"))
  (:Triggered
    (Pawn|Input|AddMovementInput (Transformation|GetActorRightVector) 1.0 false :!label _label)
    (Development|PrintString (Utilities|String|ToString(Float) ActionValue))
    (Pawn|Input|AddMovementInput (Transformation|GetActorForwardVector) 1.0 false)
    (Development|PrintString "Hello"))
  (:Started
    (goto _label)))

(event EventBeginPlay
  (Utilities|Casting|CastToPC_Player (Game|GetPlayerController 0)))

(event Collision|EventActorBeginOverlap
  (params (OtherActor :type Actor%20Object%20Reference)))

(event EventPossessed
  (params (NewController :type Controller%20Object%20Reference)))

(event EventTick
  (params (DeltaSeconds :type Float%20%28single-precision%29))
  (Transformation|AddActorWorldOffset (Math|Vector|MakeVector (* (* (Input|EnhancedActionValues|GetIA_MoveForward) (.x (Transformation|GetActorForwardVector))) 5e+01) (* (* (Input|EnhancedActionValues|GetIA_MoveSide) (.y (Transformation|GetActorRightVector))) 5e+01) 0.0)))

(fn ConstructionScript)